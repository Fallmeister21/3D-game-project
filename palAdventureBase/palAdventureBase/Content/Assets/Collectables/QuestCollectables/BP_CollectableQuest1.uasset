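; BP_CollectableQuest1 is a quest collectable actor that counts toward a quest objective when the player interacts with it.
; On interact, it checks the quest component for an active quest matching its QuestID, then adds one to the objective.
; It then flags its interactables save object as interacted, saves that to its slot and destroys itself.
; Interaction does nothing while the quest is inactive.
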(event `/Game/MarketplaceAssets/EasyQuests/Blueprints/BPI/BP_BPI_QuestsInteraction.OnInteract`
  (params (PlayerActor :type "Actor Object Reference"))
  (bind _interactablessaveobject (`self.InteractablesSaveObject`))
  (if (`/Game/MarketplaceAssets/EasyQuests/Blueprints/BP_BPC_PlayerQuestComponent.IsQuestActive?` (`self.QuestComponent`) (`self.QuestID`))
    (`/Game/MarketplaceAssets/EasyQuests/Blueprints/BP_BPC_PlayerQuestComponent.AddObjectiveAmount` (`self.QuestComponent`) (`self.QuestID`) (`self.ObjectiveID`) 1)
    (set `/Game/MarketplaceAssets/EasyQuests/Blueprints/BP_InteractablesSaveObject.HasBeenInteractedWith` true _interactablessaveobject)
    (`GameplayStatics.SaveGameToSlot` _interactablessaveobject (`self.InteractablesSaveString`))
    (`self.K2_DestroyActor`)))

(fn `UserConstructionScript`
  (`parent.UserConstructionScript`))