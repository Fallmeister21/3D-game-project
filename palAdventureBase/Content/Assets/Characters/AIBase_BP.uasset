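; AIBase_BP is a base quest character that gives quests and serves as an objective target.
; On interaction it advances matching current objectives through the quest component, or starts its assigned quests if none match.
; A text mark shows when an assigned quest can be accepted, and a world marker shows for matching marked objectives.
; BeginPlay binds to tracked-quest and completion events and hands itself to the marker widget.
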(event `self.ReceiveBeginPlay`
  (bind (_componentwasfound_ _questcomponent) (`/Game/MarketplaceAssets/EasyQuests/Blueprints/BPL/BP_BPL_Quests.GetQuestComponent`))
  (if _componentwasfound_
    (set `self.QuestComponent` _questcomponent)
    (add `/Game/MarketplaceAssets/EasyQuests/Blueprints/BP_BPC_PlayerQuestComponent.OnTrackedQuestChanged` (`self.QuestComponent`) (`|CreateDelegate` :!event `UpdateWorldMarker`))
    (`self.UpdateWorldMarker` "None")
    (`KismetSystemLibrary.Delay` 0.0)
    (add `/Game/MarketplaceAssets/EasyQuests/Blueprints/BP_BPC_PlayerQuestComponent.OnQuestCompleted` (`self.QuestComponent`) (`|CreateDelegate` :!event `UpdateQuestMark`))
    (`self.UpdateQuestMark` "None")
    (bind _aswbp_world_marker (cast `/Game/MarketplaceAssets/EasyQuests/Widgets/WBP_WorldMarker` (`WidgetComponent.GetUserWidgetObject` (`self.WorldMarker1`))))
    (set `/Game/MarketplaceAssets/EasyQuests/Widgets/WBP_WorldMarker.Actor` self _aswbp_world_marker)
    (else
      (`KismetSystemLibrary.PrintString` "Quest Component was not found." true true (struct :`R` 1.0 :`G` 0.052861 :`A` 1.0)))))

(event `self.ReceiveTick`
  (params (DeltaSeconds :type "Float (single-precision)")))

(event `/Game/MarketplaceAssets/EasyQuests/Blueprints/BPI/BP_BPI_QuestsInteraction.OnInteract`
  (params (PlayerActor :type "Actor Object Reference"))
  (bind _out (`self.Check For Any Objectives`))
  (if (not _out)
    (`/Game/MarketplaceAssets/EasyQuests/Blueprints/BP_BPC_PlayerQuestComponent.StartMultipleQuests` (`self.QuestComponent`) (`self.QuestsToAssign`))
    (`self.UpdateQuestMark` "None")
    (`self.UpdateWorldMarker` "None")))

(fn `Check For Any Objectives`
  (returns (Out :type Boolean))
  (locals (`Local Checked Any` :type Boolean))
  (for _array_element (`self.Quest IDs`)
    (bind (_foundobjective_ _foundobjectiveinfo) (`/Game/MarketplaceAssets/EasyQuests/Blueprints/BP_BPC_PlayerQuestComponent.GetCurrentObjectiveForActiveQuest` (`self.QuestComponent`) _array_element))
    (if _foundobjective_
      (for _array_element_2 (`self.Objective IDs`)
        (if (== _array_element_2 (`.Objective_ID_7_60CB1B1749DC486E0E91F796FB540B67` (break `/Game/MarketplaceAssets/EasyQuests/Blueprints/Structures/ST_Quest_Objectives` _foundobjectiveinfo)))
          (`/Game/MarketplaceAssets/EasyQuests/Blueprints/BP_BPC_PlayerQuestComponent.AddObjectiveAmount` (`self.QuestComponent`) _array_element _array_element_2 1)
          (set `local.Local Checked Any` true)))))
  (return (`local.Local Checked Any`)))

(fn `UpdateQuestMark`
  (params (`Quest ID` :type Name) (Quest :type "/Game/MarketplaceAssets/EasyQuests/Blueprints/Structures/ST_Quest_Info Structure"))
  (`SceneComponent.SetVisibility` (`self.TextRender1`) false false)
  (`/Engine/EditorBlueprintResources/StandardMacros.IsValid` (`self.QuestComponent`)
    (:`Is Valid`
      (for _array_element (`self.QuestsToAssign`)
        (if (`/Game/MarketplaceAssets/EasyQuests/Blueprints/BP_BPC_PlayerQuestComponent.CanQuestBeAccepted?` (`self.QuestComponent`) _array_element)
          (`SceneComponent.SetVisibility` (`self.TextRender1`) true false)
          (return))))))

(fn `UpdateWorldMarker`
  (params (`Quest ID` :type Name) (Quest :type "/Game/MarketplaceAssets/EasyQuests/Blueprints/Structures/ST_Quest_Info Structure"))
  (`SceneComponent.SetVisibility` (`self.WorldMarker1`) false false)
  (for _array_element (`self.Quest IDs`)
    (if (== (`.QuestID_2_E9DD1B8B405D0E58BEEA3AA29273D9A7` (break `/Game/MarketplaceAssets/EasyQuests/Blueprints/Structures/ST_Quest_Info` (`local.Quest`))) _array_element)
      (for _array_element_2 (`.Objectives_21_50C63F1D4C80B7AA25F0B7B40D0F2E3D` (break `/Game/MarketplaceAssets/EasyQuests/Blueprints/Structures/ST_Quest_Info` (`local.Quest`)))
        (bind (_foundobjective_ _foundobjectiveinfo) (`/Game/MarketplaceAssets/EasyQuests/Blueprints/BP_BPC_PlayerQuestComponent.GetCurrentObjectiveForActiveQuest` (`self.QuestComponent`) _array_element))
        (if (and (`KismetArrayLibrary.Array_Contains` (`self.Objective IDs`) (`.Objective_ID_7_60CB1B1749DC486E0E91F796FB540B67` (break `/Game/MarketplaceAssets/EasyQuests/Blueprints/Structures/ST_Quest_Objectives` _array_element_2))) (`.HasWorldMarker?_29_8F94CDC742A85DD762B02897AC787295` (break `/Game/MarketplaceAssets/EasyQuests/Blueprints/Structures/ST_Quest_Objectives` _array_element_2)) _foundobjective_ (`KismetArrayLibrary.Array_Contains` (`self.Objective IDs`) (`.Objective_ID_7_60CB1B1749DC486E0E91F796FB540B67` (break `/Game/MarketplaceAssets/EasyQuests/Blueprints/Structures/ST_Quest_Objectives` _foundobjectiveinfo))) (not (`/Game/MarketplaceAssets/EasyQuests/Blueprints/BP_BPC_PlayerQuestComponent.WasQuestAborted?` (`self.QuestComponent`) _array_element)))
          (`SceneComponent.SetVisibility` (`self.WorldMarker1`) true false)
          (return))))))

(fn `UserConstructionScript`)