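; BP_Chicken_2 is a wandering chicken pawn that players collect for a quest.
; Tick, throttled by a Delay, starts random nearby moves while idle; PawnSensing triggers a flee toward a point derived from the player's world location scaled negatively.
; Interacting while the quest is active advances the objective, saves the interacted flag, destroys the chicken and adds an item to the player's inventory.
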(event `self.PawnSensing.OnSeePawn`
  (params (Pawn :type "Pawn Object Reference"))
  (set `self.Is Moving` (`self.Is Moving`))
  (`|AIMoveTo` self (`NavigationSystemV1.K2_GetRandomLocationInNavigableRadius` (* (`self.K2_GetActorLocation` (`GameplayStatics.GetPlayerCharacter` 0)) -2) 100.0 null null) null
    (:`OnSuccess`
      (`KismetSystemLibrary.Delay` 0.5)
      (set `self.Is Moving` false))))

(event `self.ReceiveTick`
  (params (DeltaSeconds :type "Float (single-precision)"))
  (`KismetSystemLibrary.Delay` 2.0)
  (if (not (`self.Is Moving`))
    (set `self.Is Moving` true)
    (`|AIMoveTo` self (`NavigationSystemV1.K2_GetRandomReachablePointInRadius` (`self.K2_GetActorLocation`) 500.0 null null) null
      (:`OnSuccess`
        _)
      (:`OnFail`
        _))
    (set `self.Is Moving` false)))

(event `/Game/MarketplaceAssets/EasyQuests/Blueprints/BPI/BP_BPI_QuestsInteraction.OnInteract`
  (params (PlayerActor :type "Actor Object Reference"))
  (bind _interactablessaveobject (`self.InteractablesSaveObject`))
  (if (`/Game/MarketplaceAssets/EasyQuests/Blueprints/BP_BPC_PlayerQuestComponent.IsQuestActive?` (`self.QuestComponent`) (`self.QuestID`))
    (`/Game/MarketplaceAssets/EasyQuests/Blueprints/BP_BPC_PlayerQuestComponent.AddObjectiveAmount` (`self.QuestComponent`) (`self.QuestID`) (`self.ObjectiveID`) 1)
    (set `/Game/MarketplaceAssets/EasyQuests/Blueprints/BP_InteractablesSaveObject.HasBeenInteractedWith` true _interactablessaveobject)
    (`GameplayStatics.SaveGameToSlot` _interactablessaveobject (`self.InteractablesSaveString`))
    (`self.K2_DestroyActor`)
    (bind _inventorymanagercomponent (`/Game/InventorySystem/Blueprints/BPFL_InventoryFunctionLib.GetInventoryManager` (`GameplayStatics.GetPlayerCharacter` 0)))
    (`/Game/InventorySystem/Blueprints/BP_InventoryManagerComponent.AddItem` _inventorymanagercomponent "NewEnumerator8" 1)))

(fn `UserConstructionScript`
  (`parent.UserConstructionScript`))