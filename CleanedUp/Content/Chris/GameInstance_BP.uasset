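; Game instance that stores the player's stats and settings, such as turn rates, interaction range, gold, experience, level, stamina and health.
; SavePlayerInformation writes the values on its first call or when not flagged as a constructor call, so later constructor calls cannot overwrite them.
; RestorePlayerInformation returns the stored values, except mouse visibility and the being-controlled flag, which always return false.
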(fn `RestorePlayerInformation`
  (returns (BaseTurnRate :type "Float (double-precision)") (BaseLookUpRate :type "Float (double-precision)") (InterationRange :type Integer) (MouseVisibility :type Boolean) (Gold :type Integer) (Experience :type "Float (double-precision)") (ExperienceNeeded :type "Float (double-precision)") (Level :type Integer) (Stamina :type "Float (double-precision)") (Health :type "Float (double-precision)") (`IsBeingControlled?` :type Boolean) (Dummy :type Boolean))
  (return (`self.BaseTurnRate`) (`self.BaseLookUpRate`) (`self.InteractionRange`) false (`self.Gold`) (`self.Experience`) (`self.ExperienceNeeded`) (`self.Level`) (`self.Stamina`) (`self.Health`) false (`self.Dummy`)))

(fn `SavePlayerInformation`
  (params (BaseTurnRate :type "Float (double-precision)") (BaseLookUpRate :type "Float (double-precision)") (InteractionRange :type Integer) (MouseVisibility :type Boolean) (Gold :type Integer) (Experience :type "Float (double-precision)") (ExperienceNeeded :type "Float (double-precision)") (Level :type Integer) (Stamina :type "Float (double-precision)") (Health :type "Float (double-precision)") (`IsBeingControlled?` :type Boolean) (Constructor :type Boolean) (Dummy :type Boolean))
  (if (or (`self.FirstCall`) (not Constructor))
    (set `self.FirstCall` false)
    (set `self.BaseTurnRate` BaseTurnRate)
    (set `self.BaseLookUpRate` BaseLookUpRate)
    (set `self.InteractionRange` InteractionRange)
    (set `self.MouseVisibility` MouseVisibility)
    (set `self.Gold` Gold)
    (set `self.Experience` Experience)
    (set `self.ExperienceNeeded` ExperienceNeeded)
    (set `self.Level` Level)
    (set `self.Stamina` Stamina)
    (set `self.Health` Health)
    (set `self.IsBeingControlled?` `IsBeingControlled?`)
    (set `self.Dummy` Dummy)))