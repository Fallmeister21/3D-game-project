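; Wandering chicken NPC that players collect for a quest.
; Tick, throttled by a Delay, moves it to random reachable points nearby, gated by IsMoving.
; PawnSensing overrides this with a move toward a point around the player's world location times -2, apparently to flee.
; Interacting during the active quest advances the objective, saves its interacted state, destroys the actor and adds an inventory item.
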(event `self.PawnSensing.OnSeePawn`
  (params (Pawn :type "Pawn Object Reference"))
  (set `self.IsMoving` true)
  (`|AIMoveTo` null self (`NavigationSystemV1.K2_GetRandomLocationInNavigableRadius` null (* (`Actor.K2_GetActorLocation` (`GameplayStatics.GetPlayerCharacter` null)) -2) 100.0 null null) null
    (:`OnSuccess`
      (`KismetSystemLibrary.Delay` null 0.5)
      (set `self.IsMoving` false))))

(event `self.ReceiveTick`
  (params (DeltaSeconds :type "Float (single-precision)"))
  (`KismetSystemLibrary.Delay` null 2.0)
  (if (not (`self.IsMoving`))
    (set `self.IsMoving` true)
    (`|AIMoveTo` null self (`NavigationSystemV1.K2_GetRandomReachablePointInRadius` null (`Actor.K2_GetActorLocation`) 500.0 null null) null
      (:`OnSuccess`
        _)
      (:`OnFail`
        _))
    (set `self.IsMoving` false)))

(event `self.OnInteract`
  (bind _interactablessaveobject (`self.InteractablesSaveObject`))
  (if (`/Game/MarketplaceAssets/EasyQuests/Blueprints/BP_BPC_PlayerQuestComponent.IsQuestActive?` (`self.QuestComponent`) (`self.QuestID`))
    (`/Game/MarketplaceAssets/EasyQuests/Blueprints/BP_BPC_PlayerQuestComponent.AddObjectiveAmount` (`self.QuestComponent`) (`self.QuestID`) (`self.ObjectiveID`) 1)
    (set `/Game/Paul/QuestContent/BP_Chicken.HasBeenInteractedWith` true _interactablessaveobject)
    (`GameplayStatics.SaveGameToSlot` _interactablessaveobject (`self.InteractablesSaveString`))
    (`Actor.K2_DestroyActor`)
    (bind _inventorymanagercomponent (`/Game/MarketplaceAssets/InventorySystem/Blueprints/BPFL_InventoryFunctionLib.GetInventoryManager` (`GameplayStatics.GetPlayerCharacter` null)))
    (`/Game/MarketplaceAssets/InventorySystem/Blueprints/BP_InventoryManagerComponent.AddItem` _inventorymanagercomponent "NewEnumerator8" 1)))

(fn `UserConstructionScript`)