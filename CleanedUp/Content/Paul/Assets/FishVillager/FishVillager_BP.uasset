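; Fish villager Blueprint that acts as an interactable quest giver.
; On interact it calls CheckForAnyObjectives and, if that returns false, starts all of QuestsToAssign through the QuestComponent.
; It then refreshes its quest mark and world marker with a quest ID of None.
; BeginPlay, overlap and Tick are disabled stubs, and the construction script only calls the parent.
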(event `/Game/MarketplaceAssets/EasyQuests/Blueprints/BPI/BP_BPI_QuestsInteraction.OnInteract`
  (params (PlayerActor :type "Actor Object Reference"))
  (bind _out (`self.Check For Any Objectives`))
  (if (not _out)
    (`/Game/MarketplaceAssets/EasyQuests/Blueprints/BP_BPC_PlayerQuestComponent.StartMultipleQuests` (`self.QuestComponent`) (`self.QuestsToAssign`))
    (`self.UpdateQuestMark` "None")
    (`self.UpdateWorldMarker` "None")))

(fn `UserConstructionScript`
  (`parent.UserConstructionScript`))